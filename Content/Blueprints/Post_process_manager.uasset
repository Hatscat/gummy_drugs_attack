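; Post-process manager that drives screen effects when the player eats drugs, through scalar parameters in a material parameter collection.
; Each drug event, bound on BP_Player, restarts the duration timer and raises the max strength of a randomly picked effect.
; Tick shapes active effects with a sine envelope, preventing dips during ramp-up, then zeroes everything and calls DrugsEnd on the player.
; Temporary debug keys trigger or stack effects manually.
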(event Custom|playerHasEatenDrug_Event_0
  (bind _pp_effects_param_max_val (Variables|Default|Getpp_effects_param_max_val))
  ;[1 1 1] Event: eating drugs
  (Variables|Default|Setcurrent_drug_duration (Variables|Default|Getdrug_effect_base_duration))
  (bind _output_get (Variables|Default|Setrand_index (Math|Random|RandomIntegerinRange 0 (- (Variables|Default|Getarrays_length) 1))))
  (Utilities|Array|SetArrayElem _pp_effects_param_max_val _output_get (+ (Utilities|Array|Get(acopy) _pp_effects_param_max_val _output_get) 1)))

(event EventBeginPlay
  ;[1 1 1] start: seak the player event "eat drug"
  (bind _asbp_player (Utilities|Casting|CastToBP_Player (Game|GetPlayerCharacter 0)))
  (EventDispatchers|AssignPlayerHasEatenDrug _asbp_player (delegate Custom|playerHasEatenDrug_Event_0))
  ;[1 1 1] tmp
  (Input|EnableInput (Game|GetPlayerController 0)))

(event EventTick
  (params (DeltaSeconds :type Float%20%28single-precision%29))
  (bind _arrays_length (Variables|Default|Getarrays_length))
  (bind _pp_effects_param_names (Variables|Default|Getpp_effects_param_names))
  (bind _pp_effects_param_max_val (Variables|Default|Getpp_effects_param_max_val))
  (bind _pp_effects_param_current_val (Variables|Default|Getpp_effects_param_current_val))
  ;[1 1 1] Run loop
  (if (> (Variables|Default|Getcurrent_drug_duration) 0.0)
    (Variables|Default|Setcurrent_drug_duration (- (Variables|Default|Getcurrent_drug_duration) DeltaSeconds))
    (for _index (range 0 _arrays_length)
      (if (!= (Utilities|Array|Get(acopy) _pp_effects_param_max_val _index) 0)
        (if (and (> (/ (Variables|Default|Getcurrent_drug_duration) (Variables|Default|Getdrug_effect_base_duration)) 0.5) (< (* (Utilities|Array|Get(acopy) _pp_effects_param_max_val _index) (Math|Trig|Sin(Radians) (Math|Float|MultiplybyPi (/ (Variables|Default|Getcurrent_drug_duration) (Variables|Default|Getdrug_effect_base_duration))))) (Utilities|Array|Get(acopy) _pp_effects_param_current_val _index)))
          (Utilities|Array|SetArrayElem _pp_effects_param_current_val _index (Utilities|Array|Get(acopy) _pp_effects_param_current_val _index))
          (Rendering|Material|SetScalarParameterValue "/Game/Materials/post_process_collection.post_process_collection" (Utilities|String|StringToName (Utilities|Array|Get(acopy) _pp_effects_param_names _index)) (Utilities|Array|Get(acopy) _pp_effects_param_current_val _index) :!class /Script/Engine.KismetMaterialLibrary)
          (else
            (Utilities|Array|SetArrayElem _pp_effects_param_current_val _index (* (Utilities|Array|Get(acopy) _pp_effects_param_max_val _index) (Math|Trig|Sin(Radians) (Math|Float|MultiplybyPi (/ (Variables|Default|Getcurrent_drug_duration) (Variables|Default|Getdrug_effect_base_duration))))))
            (Rendering|Material|SetScalarParameterValue "/Game/Materials/post_process_collection.post_process_collection" (Utilities|String|StringToName (Utilities|Array|Get(acopy) _pp_effects_param_names _index)) (* (Utilities|Array|Get(acopy) _pp_effects_param_max_val _index) (Math|Trig|Sin(Radians) (Math|Float|MultiplybyPi (/ (Variables|Default|Getcurrent_drug_duration) (Variables|Default|Getdrug_effect_base_duration))))) :!class /Script/Engine.KismetMaterialLibrary)))))
    (elif (!= (Variables|Default|Getrand_index) -1)
      (Variables|Default|Setrand_index -1)
      (for _index_2 (range 0 _arrays_length)
        (Utilities|Array|SetArrayElem _pp_effects_param_current_val _index_2 0.0)
        (Utilities|Array|SetArrayElem _pp_effects_param_max_val _index_2 0)
        (Rendering|Material|SetScalarParameterValue "/Game/Materials/post_process_collection.post_process_collection" (Utilities|String|StringToName (Utilities|Array|Get(acopy) _pp_effects_param_names _index_2)) 0.0 :!class /Script/Engine.KismetMaterialLibrary))
      (Default|DrugsEnd (stale EventBeginPlay _asbp_player)))))

(event Input|KeyboardEvents|Ampersand
  (bind _pp_effects_param_max_val (Variables|Default|Getpp_effects_param_max_val))
  ;[1 1 1] tmp
  (:Pressed
    (Utilities|Array|SetArrayElem _pp_effects_param_max_val 0 (+ (Utilities|Array|Get(acopy) _pp_effects_param_max_val) 1))
    (Variables|Default|Setcurrent_drug_duration (Variables|Default|Getdrug_effect_base_duration))
    (Variables|Default|Setrand_index 1)))

(event Input|KeyboardEvents|EAccentAigu
  (bind _pp_effects_param_max_val (Variables|Default|Getpp_effects_param_max_val))
  ;[1 1 1] tmp
  (:Pressed
    (Utilities|Array|SetArrayElem _pp_effects_param_max_val 1 (+ (Utilities|Array|Get(acopy) _pp_effects_param_max_val 1) 1))
    (Variables|Default|Setcurrent_drug_duration (Variables|Default|Getdrug_effect_base_duration))
    (Variables|Default|Setrand_index 1)))

(event Input|KeyboardEvents|Add
  ;[1 1 1] tmp
  (:Pressed
    (CallFunction|PlayerHasEatenDrugEvent0)))

(fn ConstructionScript
  (bind _pp_effects_param_names (Variables|Default|Getpp_effects_param_names))
  (bind _returnvalue (Utilities|Array|Length _pp_effects_param_names))
  (Utilities|Array|Resize (Variables|Default|Getpp_effects_param_max_val) _returnvalue)
  (Utilities|Array|Resize (Variables|Default|Getpp_effects_param_current_val) _returnvalue)
  (Variables|Default|Setarrays_length _returnvalue))