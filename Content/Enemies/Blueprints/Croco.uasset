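; Croco is an enemy Blueprint whose construction script only calls its parent's, so any active setup in this graph comes from the parent class.
; Disconnected leftover nodes, which never run, would assign a star mesh and wireframe core material, disable collision, and create a tinted dynamic enemy material with no throb and raised brightness.
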(fn ConstructionScript
  (|CallParentFunction))