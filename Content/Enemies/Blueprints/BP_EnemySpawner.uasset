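; Enemy spawner that runs escalating timed waves, creating random enemies at random spawn points while the player is alive.
; Looping timers advance the GeoGameState wave, grow the enemy quota and spawn rate (capped), and unlock enemy types at wave thresholds.
; Spawning pauses when the never-reset spawn count equals the quota; a spawn tick finding the player dead clears all timers.
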(event Custom|nextWave
  (bind _geogame (Variables|Default|GetGeoGame))
  ;[0.01177 1 0] next wave
  (Variables|/Game/Game/GeoGameState.GeoGameState_C|SetActiveWave _geogame (+ (Variables|/Game/Game/GeoGameState.GeoGameState_C|GetActiveWave _geogame) 1))
  (Variables|Default|SetwavesEneniesNb (+ (Variables|Default|GetwavesEneniesNb) (Math|Float|Floor (* (Variables|Default|GetwavesEneniesNb) (Variables|Default|GetwavesNbMult)))))
  (bind _output_get (Variables|Default|SetenemiesPerSecond (Math|Float|Min(Float) (+ (Variables|Default|GetenemiesPerSecond) (Variables|Default|GetenemyRateIncrease)) 6e+01)))
  (Utilities|Time|SetTimerbyFunctionName 0 "spawnEnemy" (/ 1.0 _output_get) true))

(event Custom|spawnEnemy
  (bind _spawnpoints (Variables|Default|GetspawnPoints))
  ;[1 0.7555 0] spawn
  (if (Variables|/Game/Game/GeoGameState.GeoGameState_C|GetPlayerAlive (Variables|Default|GetGeoGame))
    (Game|SpawnActorfromClass (Utilities|Array|Get(acopy) (Variables|Default|Getenemies) (Math|Random|RandomIntegerinRange 0 (Variables|Default|GetcurEnemyMaxType))) (Transformation|GetActorTransform (Utilities|Array|Get(acopy) _spawnpoints (Math|Random|RandomInteger (Utilities|Array|Length _spawnpoints)))) false "(R=1.000000,G=0.005134,B=0.000000,A=1.000000)" 0)
    (bind _output_get (Variables|Default|SetcurEnemySpawnedNb (+ 1 (Variables|Default|GetcurEnemySpawnedNb))))
    (if (== _output_get (Variables|Default|GetwavesEneniesNb))
      (Utilities|Time|ClearTimerbyFunctionName 0 "spawnEnemy"))
    (else
      (CallFunction|GameIsEnding))))

(event Custom|checkMaxEnemyType
  (bind _enemieswaverequired (Variables|Default|GetenemiesWaveRequired))
  ;[0.01177 1 0] Check for max enemy type
  (if (and (< (Variables|Default|GetcurEnemyMaxType) (- (Utilities|Array|Length _enemieswaverequired) 1)) (<= (Utilities|Array|Get(acopy) _enemieswaverequired (Variables|Default|GetcurEnemyMaxType)) (Variables|/Game/Game/GeoGameState.GeoGameState_C|GetActiveWave (Variables|Default|GetGeoGame))))
    (Variables|Default|SetcurEnemyMaxType (+ (Variables|Default|GetcurEnemyMaxType) 1))))

(event Custom|gameIsEnding
  ;[0 0 0] Stop
  (Utilities|Time|ClearTimerbyFunctionName 0 "checkMaxEnemyType")
  (Utilities|Time|ClearTimerbyFunctionName 0 "nextWave")
  (Utilities|Time|ClearTimerbyFunctionName 0 "spawnEnemy"))

(event EventBeginPlay
  ;[0.07873 0.07718 1] Init
  (bind _asgeo_game_state (Utilities|Casting|CastToGeoGameState (Game|GetGameState)))
  (Variables|Default|SetGeoGame _asgeo_game_state)
  (CallFunction|NextWave)
  (Utilities|Time|SetTimerbyFunctionName 0 "checkMaxEnemyType" 1.0 true)
  (Utilities|Time|SetTimerbyFunctionName 0 "nextWave" (Variables|Default|GetwavesInterval) true)
  (bind _asbp_player (Utilities|Casting|CastToBP_Player (Game|GetPlayerCharacter 0)))
  (Variables|Default|SetMyPlayer _asbp_player))

(fn ConstructionScript)