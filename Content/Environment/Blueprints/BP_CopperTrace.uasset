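; BP_CopperTrace is an environment Blueprint that builds a copper trace as meshes along a spline.
; The construction script divides the TraceSpline length by SplineSpace to set the loop count, adding a spline mesh component each iteration.
; Each mesh takes its start and end positions and tangents from consecutive spline points, indexed by the loop counter rather than by distance along the spline.
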(fn ConstructionScript
  (bind _tracespline (Variables|Default|GetTraceSpline))
  (for _index (range 0 (.ReturnValue (Math|Float|Division(WholeandRemainder) (Spline|GetSplineLength (Variables|Default|GetTraceSpline)) (Variables|Default|GetSplineSpace))))
    (bind _returnvalue (AddComponent|AddSplineMeshComponent false))
    (SplineMesh|SetStartandEnd _returnvalue (.LocalLocation (Class|SplineComponent|GetLocalLocationandTangentatSplinePoint _tracespline _index)) (.LocalTangent (Class|SplineComponent|GetLocalLocationandTangentatSplinePoint _tracespline _index)) (.LocalLocation (Class|SplineComponent|GetLocalLocationandTangentatSplinePoint _tracespline (+ _index 1))) (.LocalTangent (Class|SplineComponent|GetLocalLocationandTangentatSplinePoint _tracespline (+ _index 1))) :!class /Script/Engine.SplineMeshComponent)))